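; BP_Axe is an axe pickup that grants the player the axe.
; Overlap events on its Trigger component track whether something is near the axe, without filtering which actor overlaps.
; Pressing F while near sets HacheObtenue on the third-person character, shows a Level 1 HUD message hinting that the axe breaks wooden doors, then destroys the actor.
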(event `self.Trigger.OnComponentBeginOverlap`
  (params (OverlappedComponent :type "PrimitiveComponent Object Reference") (OtherActor :type "Actor Object Reference") (OtherComp :type "PrimitiveComponent Object Reference") (OtherBodyIndex :type Integer) (bFromSweep :type Boolean) (SweepResult :type "HitResult Structure (by ref)"))
  ; Vérifie si la hache est ramassable ou non.
  (set `self.Hache proche` true))

(event `self.Trigger.OnComponentEndOverlap`
  (params (OverlappedComponent :type "PrimitiveComponent Object Reference") (OtherActor :type "Actor Object Reference") (OtherComp :type "PrimitiveComponent Object Reference") (OtherBodyIndex :type Integer))
  ; Vérifie si la hache est ramassable ou non.
  (set `self.Hache proche` false))

(event `Key|F` :consume false
  (params (Key :type "Key Structure"))
  ; Ramasse la hache avec la touche "F" et fait apparaître un message dans le HUD.
  (:`Pressed`
    (if (`self.Hache proche`)
      (bind _asbp_third_person_character (cast `/Game/ThirdPerson/Blueprints/BP_ThirdPersonCharacter` (`GameplayStatics.GetPlayerPawn` 0)))
      (set `/Game/ThirdPerson/Blueprints/BP_ThirdPersonCharacter.Hache obtenue` true _asbp_third_person_character)
      (bind _asbp_hud_lvl_1 (cast `/Game/Game/Blueprints/Interfaces/BP_HUD_Lvl1` (`PlayerController.GetHUD` (`GameplayStatics.GetPlayerController` 0))))
      (`TextBlock.SetText` (`/Game/Game/Blueprints/Interfaces/BP_HUD_Lvl1.Main Message` _asbp_hud_lvl_1) "Cette hache devrait te permettre de détruire les portes en bois. (Mais qu'est-ce que ça fait là dans un sous-marin!?)")
      (`self.K2_DestroyActor`))))

(fn `UserConstructionScript`)