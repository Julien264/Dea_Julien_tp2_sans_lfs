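; BP_keyCard is a keycard pickup that grants the player the key to the submarine's exit.
; Overlap events on its Trigger component set a proximity flag, without filtering which actor overlaps.
; Pressing F while the flag is set marks the key as obtained on BP_ThirdPersonCharacter.
; It then shows a French message in BP_HUD_Lvl1 directing the player to the red exit door, plays a sound and destroys itself.
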(event `self.Trigger.OnComponentBeginOverlap`
  (params (OverlappedComponent :type "PrimitiveComponent Object Reference") (OtherActor :type "Actor Object Reference") (OtherComp :type "PrimitiveComponent Object Reference") (OtherBodyIndex :type Integer) (bFromSweep :type Boolean) (SweepResult :type "HitResult Structure (by ref)"))
  ; Vérifie si la carte est proche ou non.
  (set `self.KeyCard proche` true))

(event `self.Trigger.OnComponentEndOverlap`
  (params (OverlappedComponent :type "PrimitiveComponent Object Reference") (OtherActor :type "Actor Object Reference") (OtherComp :type "PrimitiveComponent Object Reference") (OtherBodyIndex :type Integer))
  ; Vérifie si la carte est proche ou non.
  (set `self.KeyCard proche` false))

(event `Key|F` :consume false
  (params (Key :type "Key Structure"))
  ; Ramasse la carte avec la touche "F" et fait apparaître un message dans le HUD.
  (:`Pressed`
    (if (`self.KeyCard proche`)
      (bind _asbp_third_person_character (cast `/Game/ThirdPerson/Blueprints/BP_ThirdPersonCharacter` (`GameplayStatics.GetPlayerPawn` 0)))
      (set `/Game/ThirdPerson/Blueprints/BP_ThirdPersonCharacter.KeyCard obtenue` true _asbp_third_person_character)
      (bind _asbp_hud_lvl_1 (cast `/Game/Game/Blueprints/Interfaces/BP_HUD_Lvl1` (`PlayerController.GetHUD` (`GameplayStatics.GetPlayerController` 0))))
      (`TextBlock.SetText` (`/Game/Game/Blueprints/Interfaces/BP_HUD_Lvl1.Main Message` _asbp_hud_lvl_1) "C'est la clé pour la sortie du sous-marin. Va à la grande porte rouge et sort. Il est déjà à la surface.")
      (`GameplayStatics.PlaySound2D` "/Game/Game/Audio/cle_electrique.cle_electrique" 1.0 1.0 0.0 null null)
      (`self.K2_DestroyActor`))))

(fn `UserConstructionScript`)