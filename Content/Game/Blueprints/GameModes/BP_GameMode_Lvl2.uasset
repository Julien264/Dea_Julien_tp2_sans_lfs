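; Game mode for level 2 that tracks a piece counter and decides when a weapon becomes purchasable.
; BeginPlay resets the counter and enables input from the first player controller, letting the R key restart the level through a console command.
; AugmenterPiece increments the counter and sets the ArmeAchetable flag when it reaches exactly three.
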(event `self.ReceiveBeginPlay`
  (set `self.Nombre de piece` 0)
  (`self.EnableInput` (`GameplayStatics.GetPlayerController` 0)))

(event `Key|R`
  (params (Key :type "Key Structure"))
  (:`Pressed`
    (`KismetSystemLibrary.ExecuteConsoleCommand` "Restartlevel" null)))

(fn `AugmenterPiece`
  (set `self.Nombre de piece` (+ (`self.Nombre de piece`) 1))
  (`/Engine/EditorBlueprintResources/StandardMacros.CompareInt` (`self.Nombre de piece`) 3
    (:`==`
      (set `self.Arme achetable` true))))

(fn `UserConstructionScript`)