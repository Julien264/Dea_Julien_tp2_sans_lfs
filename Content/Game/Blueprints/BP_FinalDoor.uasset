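; BP_FinalDoor is a level-exit door that sends the player to the Lvl_2_port level once they hold the key card.
; A Trigger component's begin and end overlaps, unfiltered by actor, set a PorteProche proximity flag.
; Pressing F while the flag is set checks KeyCardObtenue on the player's BP_ThirdPersonCharacter, then calls ChangerNiveau on BP_GameInstance.
; Without the card, it prints "Not yet" and plays an access-denied sound.
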(event `self.Trigger.OnComponentBeginOverlap`
  (params (OverlappedComponent :type "PrimitiveComponent Object Reference") (OtherActor :type "Actor Object Reference") (OtherComp :type "PrimitiveComponent Object Reference") (OtherBodyIndex :type Integer) (bFromSweep :type Boolean) (SweepResult :type "HitResult Structure (by ref)"))
  (set `self.Porte proche` true))

(event `self.Trigger.OnComponentEndOverlap`
  (params (OverlappedComponent :type "PrimitiveComponent Object Reference") (OtherActor :type "Actor Object Reference") (OtherComp :type "PrimitiveComponent Object Reference") (OtherBodyIndex :type Integer))
  (set `self.Porte proche` false))

(event `Key|F` :consume false
  (params (Key :type "Key Structure"))
  (:`Pressed`
    (if (`self.Porte proche`)
      (bind _asbp_third_person_character (cast `/Game/ThirdPerson/Blueprints/BP_ThirdPersonCharacter` (`GameplayStatics.GetPlayerPawn` 0)))
      (if (`/Game/ThirdPerson/Blueprints/BP_ThirdPersonCharacter.KeyCard obtenue` _asbp_third_person_character)
        (bind _asbp_game_instance (cast `/Game/Game/Systems/BP_GameInstance` (`GameplayStatics.GetGameInstance`)))
        (`/Game/Game/Systems/BP_GameInstance.ChangerNiveau` _asbp_game_instance "Lvl_2_port" (make `SoftWorldReference` "/Game/Game/Maps/Lvl_2_port.Lvl_2_port"))
        (else
          (`KismetSystemLibrary.PrintString` "Not yet")
          (`GameplayStatics.PlaySound2D` "/Game/Game/Audio/access_denied.access_denied" 1.0 1.0 0.0 null null))))))

(fn `UserConstructionScript`)